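; BP_Test is a test Blueprint that prints a fixed message on BeginPlay and manipulates an integer counter, MyVar, through keys.
; X prints the counter, while C and Z both increment it by one, Z by subtracting negative one.
; C prints the sum recomputed from the updated value, so its output reads one higher than the stored counter.
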(event `self.ReceiveBeginPlay`
  (`KismetSystemLibrary.PrintText` "MEGUH MERN"))

(event `Key|X`
  (params (Key :type "Key Structure" :default "AnyKey"))
  (:`Pressed`
    (`KismetSystemLibrary.PrintText` (`KismetTextLibrary.Conv_IntToText` (`self.MyVar`)))))

(event `self.ReceiveActorBeginOverlap`
  (params (OtherActor :type "Actor Object Reference")))

(event `self.ReceiveTick`
  (params (DeltaSeconds :type "Float (single-precision)")))

(event `Key|C`
  (params (Key :type "Key Structure" :default "AnyKey"))
  (bind _returnvalue (+ (`self.MyVar`) 1 0))
  (:`Pressed`
    (set `self.MyVar` _returnvalue)
    (`KismetSystemLibrary.PrintText` (`KismetTextLibrary.Conv_IntToText` _returnvalue))))

(event `Key|Z`
  (params (Key :type "Key Structure" :default "AnyKey"))
  (:`Pressed`
    (bind _output_get (set `self.MyVar` (- (`self.MyVar`) -1)))
    (`KismetSystemLibrary.PrintText` (`KismetTextLibrary.Conv_IntToText` _output_get))))

(fn `UserConstructionScript`)