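; BP_Switch is a trigger actor that randomly recolors a chair when another actor starts or stops overlapping it.
; The construction script creates a dynamic material instance on the Chair component's first material slot and stores it as Color.
; Both overlap events write a new random RGB value to that instance's ColorSeats parameter.
; BeginPlay prints a creation message.
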(event `self.ReceiveBeginPlay`
  (`KismetSystemLibrary.PrintText` "BP_Switch Created"))

(event `self.ReceiveActorBeginOverlap`
  (params (OtherActor :type "Actor Object Reference"))
  (`MaterialInstanceDynamic.SetVectorParameterValue` (`self.Color`) "ColorSeats" (`KismetMathLibrary.MakeColor` (`KismetMathLibrary.RandomFloatInRange` 0.0 1.0) (`KismetMathLibrary.RandomFloatInRange` 0.0 1.0) (`KismetMathLibrary.RandomFloatInRange` 0.0 1.0))))

(event `self.ReceiveActorEndOverlap`
  (params (OtherActor :type "Actor Object Reference"))
  (`MaterialInstanceDynamic.SetVectorParameterValue` (`self.Color`) "ColorSeats" (`KismetMathLibrary.MakeColor` (`KismetMathLibrary.RandomFloatInRange` 0.0 1.0) (`KismetMathLibrary.RandomFloatInRange` 0.0 1.0) (`KismetMathLibrary.RandomFloatInRange` 0.0 1.0))))

(fn `UserConstructionScript`
  (bind _returnvalue (`PrimitiveComponent.CreateDynamicMaterialInstance` (`self.chair`) 0 null))
  (set `self.Color` _returnvalue))